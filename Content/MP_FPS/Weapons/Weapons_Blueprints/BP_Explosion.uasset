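; BP_Explosion is an explosion actor, apparently for grenades, that kills characters caught in its collision sphere.
; On BeginPlay it activates its particles and explosion sound, then removes the sphere after a short delay.
; Any overlap replays the effects, and BP_Character_Master actors receive ServerKillPlayer, with no damage falloff.
; The DestroyActor nodes are unwired, so the graph never destroys the actor itself.
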(event OnComponentBeginOverlap(Sphere_Collision)
  (params (OverlappedComponent :type Primitive%20Component%20Object%20Reference) (OtherActor :type Actor%20Object%20Reference) (OtherComp :type Primitive%20Component%20Object%20Reference) (OtherBodyIndex :type Integer) (bFromSweep :type Boolean) (SweepResult :type Hit%20Result%20Structure%20%28by%20ref%29))
  (Components|Activation|Activate (Variables|Default|GetParticleSystem) false)
  (Audio|PlaySoundatLocation "/Game/MP_FPS/MilitaryWeapSilver/Sound/GrenadeLauncher/Wavs/GrenadeLauncher_Explosion01.GrenadeLauncher_Explosion01" (Transformation|GetActorLocation))
  (bind _asbp_character_master (Utilities|Casting|CastToBP_Character_Master OtherActor))
  (Default|ServerKillPlayer _asbp_character_master))

(event EventBeginPlay
  (Components|Activation|Activate (Variables|Default|GetParticleSystem) false)
  (Audio|PlaySoundatLocation "/Game/MP_FPS/MilitaryWeapSilver/Sound/GrenadeLauncher/Wavs/GrenadeLauncher_Explosion01.GrenadeLauncher_Explosion01" (Transformation|GetActorLocation))
  (Utilities|FlowControl|Delay 2.0)
  (Development|PrintString "se desactiva granada")
  (Components|DestroyComponent (Variables|Default|GetSphere_Collision)))

(fn ConstructionScript)