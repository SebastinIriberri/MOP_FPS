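; Multiplayer FPS game mode that handles player respawning at random player starts.
; Two seconds after BeginPlay, the authority caches every PlayerStart actor in an array.
; Server_RespawnPlayer spawns a BP_Character_Master, adjusting for collisions but always spawning, and has the given PlayerController possess it.
; Spawn location and rotation come from separate random picks, so they can belong to different starts.
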(event Custom|Server_RespawnPlayer
  (params (PlayerController :type Player%20Controller%20Object%20Reference))
  (bind _playerstarts (Variables|Default|GetPlayerStarts))
  (bind _returnvalue (Utilities|Array|Length _playerstarts))
  (bind _returnvalue_2 (- _returnvalue 1))
  (bind _returnvalue_3 (Math|Random|RandomIntegerinRange _returnvalue_2 0))
  (bind _item (Utilities|Array|Get(acopy) _playerstarts _returnvalue_3))
  (bind _returnvalue_4 (Transformation|GetActorTransform _item))
  (Utilities|IsValid PlayerController
    (:Is%20Valid
      (bind _returnvalue_5 (Game|SpawnActorfromClass "/Game/MP_FPS/Characters/Blueprints/BP_Character_Master.BP_Character_Master_C" (Math|Transform|MakeTransform (.location _returnvalue_4) (.rotation _returnvalue_4) "1,1,1") "AdjustIfPossibleButAlwaysSpawn" 0 0))
      (Utilities|IsValid _returnvalue_5
        (:Is%20Valid
          (Pawn|Possess PlayerController _returnvalue_5))))))

(event EventBeginPlay
  (Utilities|FlowControl|Delay 2.0)
  (Networking|SwitchHasAuthority
    (:Authority
      (bind _outactors (Actor|GetAllActorsOfClass "/Script/Engine.PlayerStart"))
      (for _array_element _outactors
        (Utilities|Array|Add (Variables|Default|GetPlayerStarts) _array_element)))))

(fn ConstructionScript)