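; Game instance for the multiplayer FPS that handles menu display and starting single-player or hosted games.
; Events create and show the main and multiplayer menu widgets, with the multiplayer menu switching to UI-only input.
; Single-player opens the test map directly, while hosting creates a non-LAN session and reopens that map as a listen server.
; Both starts set game-only input, but hosting leaves the mouse cursor visible.
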(event Custom|ShowMultiplayerMenu
  (bind _returnvalue (Game|GetPlayerController 0))
  (bind _returnvalue_2 (UserInterface|CreateWidget "/Game/MP_FPS/Widgets/UI/BPW_MultiplayerMenu.BPW_MultiplayerMenu_C" _returnvalue))
  (Variables|Default|SetMultiplayer%20Menu%20ref _returnvalue_2)
  (UserInterface|Viewport|AddtoViewport (Variables|Default|GetMultiplayer%20Menu%20ref) 0)
  (Input|SetInputModeUIOnly _returnvalue (Variables|Default|GetMultiplayer%20Menu%20ref) "DoNotLock")
  (Variables|/Script/Engine.PlayerController|SetbShowMouseCursor _returnvalue true))

(event Custom|StartSinglePlayer
  (bind _returnvalue (Game|GetPlayerController 0))
  (Game|OpenLevel(byName) "Test_Map_001")
  (Input|SetInputModeGameOnly _returnvalue)
  (Variables|/Script/Engine.PlayerController|SetbShowMouseCursor _returnvalue false))

(event Custom|HostGame
  (bind _returnvalue (Game|GetPlayerController 0))
  (|Session _returnvalue 10 false
    (:OnSuccess
      (Game|OpenLevel(byName) "Test_Map_001" true "listen")
      (Input|SetInputModeGameOnly _returnvalue)
      (Variables|/Script/Engine.PlayerController|SetbShowMouseCursor _returnvalue true))
    (:OnFailure
      (Development|PrintString "Host Game Failed"))))

(event Custom|ShowMainMenu
  (bind _returnvalue (UserInterface|CreateWidget "/Game/MP_FPS/Widgets/UI/BPW_MainMenu.BPW_MainMenu_C" (Game|GetPlayerController 0)))
  (Variables|Default|SetMainmenuRef _returnvalue)
  (UserInterface|Viewport|AddtoViewport (Variables|Default|GetMainmenuRef) 0))